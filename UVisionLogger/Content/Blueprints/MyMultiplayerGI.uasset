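; Multiplayer game instance that creates, finds and joins LAN sessions.
; Creating a session enables VR, then opens the map set by MapChangeEvent as a listen server.
; Finding stores the results and passes their count to the MainMenuHUD.
; Joining always takes the first stored session, then unpauses the game on the client two seconds after success.
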(event `self.MapChangeEvent`
  (params (s :type String))
  ;[1 1 1] map name changed
  (set `self.MapName` s))

(event `self.CreateSessionEvent`
  ;[1 1 1] create lobby
  ;[1 1 1] turn on vr
  (`HeadMountedDisplayFunctionLibrary.EnableHMD` true)
  (`KismetSystemLibrary.PrintString` "VR on")
  (`CreateSessionCallbackProxy.CreateSession` (`GameplayStatics.GetPlayerController` 0) 10 true
    (:`OnSuccess`
      (`GameplayStatics.OpenLevel` (`KismetStringLibrary.Conv_StringToName` (`self.MapName`)) true "listen")
      (`KismetSystemLibrary.PrintString` "level opened"))
    (:`OnFailure`
      (`KismetSystemLibrary.PrintString` "failed to create session"))))

(event `self.JoinSessionEvent`
  ;[1 1 1] join session
  (if (> (`self.NumberOfSessions`) 0)
    (`JoinSessionCallbackProxy.JoinSession` (`GameplayStatics.GetPlayerController` 0) (`|GetArrayItem` (`self.Sessions`))
      (:`OnSuccess`
        (`KismetSystemLibrary.PrintString` "joined session")
        ;[1 1 1] unpause game for client
        (`KismetSystemLibrary.Delay` 2.0)
        (`GameplayStatics.SetGamePaused` false)
        (`KismetSystemLibrary.PrintString` "unpaused"))
      (:`OnFailure`
        (`KismetSystemLibrary.PrintString` "failed to join session")))
    (else
      (`KismetSystemLibrary.PrintString` "no session to join"))))

(event `self.FindSessionEvent`
  (bind _returnvalue (`GameplayStatics.GetPlayerController` 0))
  ;[1 1 1] find session
  (bind _results (`FindSessionsCallbackProxy.FindSessions` _returnvalue 10 true)
    (:`OnSuccess`
      (bind _output_get (set `self.NumberOfSessions` (`KismetArrayLibrary.Array_Length` _results)))
      (if (> _output_get 0)
        (`KismetSystemLibrary.PrintString` "sessions found")
        (set `self.Sessions` _results)
        (bind _asmain_menu_hud (cast `MainMenuHUD` (`PlayerController.GetHUD` _returnvalue)))
        (`MainMenuHUD.GiveSessionsNumber` _asmain_menu_hud (`self.NumberOfSessions`))
        (else
          (`KismetSystemLibrary.PrintString` "no sessions found" :!label _label))))
    (:`OnFailure`
      (goto _label))))